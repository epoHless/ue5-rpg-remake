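; BP_Player is the player entity Blueprint, which keeps a HeldItem sprite in sync with the current inventory item.
; On BeginPlay it binds the inventory's slot-changed, item-added and item-removed events to SetHeldItem.
; When the slot's item matches the current item, that function shows the item's sprite, or makes HeldItem transparent if the item is invalid.
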(event Custom|OnSlotChanged_Event
  (params (Slot :type Inventory%20Slot%20Object%20Reference) (Index :type Integer))
  (CallFunction|SetHeldItem Slot))

(event Custom|OnItemRemoved_Event
  (params (Slot :type Inventory%20Slot%20Object%20Reference) (Index :type Integer))
  (CallFunction|SetHeldItem Slot))

(event Custom|OnItemAdded_Event
  (params (Slot :type Inventory%20Slot%20Object%20Reference) (Index :type Integer))
  (CallFunction|SetHeldItem Slot))

(event EventBeginPlay
  (bind _returnvalue (Class|PlayerEntity|GetInventory))
  (|CallParentFunction)
  (EventDispatchers|AssignOnSlotChanged _returnvalue (delegate Custom|OnSlotChanged_Event))
  (EventDispatchers|AssignOnItemRemoved _returnvalue (delegate Custom|OnItemRemoved_Event))
  (EventDispatchers|AssignOnItemAdded _returnvalue (delegate Custom|OnItemAdded_Event)))

(fn ConstructionScript)

(fn SetHeldItem
  (params (Slot :type Inventory%20Slot%20Object%20Reference))
  (bind _item (Variables|/Script/EntitySystem.InventorySlot|GetItem Slot))
  (if (== (Variables|/Script/EntitySystem.InventorySlot|GetItem Slot) (Class|Inventory|GetCurrentItem (Class|PlayerEntity|GetInventory)))
    (Utilities|IsValid _item
      (:Is%20Valid
        (Sprite|SetSpriteColor (Variables|Default|GetHeldItem) "(R=1.000000,G=1.000000,B=1.000000,A=1.000000)")
        (Rendering|Components|Sprite|SetSprite (Variables|Default|GetHeldItem) (Variables|/Script/EntitySystem.Item|GetSprite _item)))
      (:Is%20Not%20Valid
        (Sprite|SetSpriteColor (Variables|Default|GetHeldItem) "(R=0.000000,G=0.000000,B=0.000000,A=0.000000)")))))
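; BP_Enemy is an enemy character with a sprite, a widget health bar, and feedback when it takes damage.
; On BeginPlay it caches the HP bar widget and binds health and damage events, so health changes update the bar's percentage.
; Damage triggers a timeline that tints the sprite between white and dark red, and launches the enemy opposite its current velocity as knockback.
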(event Custom|OnHealthChanged_Event
  (params (Percentage :type Float%20%28single-precision%29))
  (Progress|SetPercent (Variables|/Game/Core/Blueprints/UI/Entities/UW_EntityHPBar.UW_EntityHPBar_C|GetHPBar (stale EventBeginPlay _output_get)) Percentage))

(event Custom|OnDamageTaken_Event
  (params (Percentage :type Float%20%28single-precision%29))
  (CallFunction|OnHit)
  (Character|LaunchCharacter (* (* (Math|Vector|Normalize (Variables|/Script/Engine.MovementComponent|GetVelocity (Pawn|GetMovementComponent))) (Math|Conversions|ToVector(Float) -1.0)) (Math|Conversions|ToVector(Float) 7e+01)) true false))

(event Custom|On%20Hit
  (bind _value (Timeline|Timeline PlayFromStart)
    (:Update
      (Sprite|SetSpriteColor (Variables|Default|GetSprite) (Math|Color|Lerp(LinearColor) "(R=1.000000,G=1.000000,B=1.000000,A=1.000000)" "(R=0.526042,G=0.000000,B=0.012556,A=1.000000)" _value)))))

(event EventBeginPlay
  (|CallParentFunction)
  (bind _asuw_entity_hpbar (Utilities|Casting|CastToUW_EntityHPBar (UserInterface|GetWidget (Variables|Default|GetWidget))))
  (bind _output_get (Variables|Default|SetHP%20Bar _asuw_entity_hpbar))
  (EventDispatchers|AssignOnHealthChanged (delegate Custom|OnHealthChanged_Event))
  (EventDispatchers|AssignOnDamageTaken (delegate Custom|OnDamageTaken_Event)))

(fn ConstructionScript)
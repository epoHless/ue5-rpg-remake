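; BP_Bound is a Blueprint that animates an arrow sprite sliding back and forth along a set direction, apparently as a visual bound indicator.
; On BeginPlay it caches the sprite's relative location and computes an end point from MovementDirection scaled by Multiplier.
; The Locomotion timeline lerps the sprite between the two points, and its Finished output alternates reverse and forward playback for an endless ping-pong loop.
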(event Custom|Play%20FW
  (bind (_direction _value) (Timeline|Locomotion PlayFromStart)
    (:Update
      (Transformation|SetRelativeLocation (Variables|Default|GetArrow%20Sprite) (Math|Vector|Lerp(Vector) (Variables|Default|GetStart%20Location) (Variables|Default|GetEnd%20Location) _value) false false))
    (:Finished
      (switch Utilities|FlowControl|Switch|SwitchonETimelineDirection _direction
        (:Forward
          (CallFunction|PlayRW))
        (:Backward
          (CallFunction|PlayFW))))))

(event Custom|Play%20RW
  (bind (_direction _value) (Timeline|Locomotion ReverseFromEnd)
    (:Update
      (Transformation|SetRelativeLocation (Variables|Default|GetArrow%20Sprite) (Math|Vector|Lerp(Vector) (Variables|Default|GetStart%20Location) (Variables|Default|GetEnd%20Location) _value) false false))
    (:Finished
      (switch Utilities|FlowControl|Switch|SwitchonETimelineDirection _direction
        (:Forward
          (CallFunction|PlayRW))
        (:Backward
          (CallFunction|PlayFW))))))

(event EventBeginPlay
  (Variables|Default|SetStart%20Location (Variables|/Script/Engine.SceneComponent|GetRelativeLocation (Variables|Default|GetArrow%20Sprite)))
  (Variables|Default|SetEnd%20Location (CallFunction|GetEndLocation 1.0))
  (bind (_direction _value) (Timeline|Locomotion Play)
    (:Update
      (Transformation|SetRelativeLocation (Variables|Default|GetArrow%20Sprite) (Math|Vector|Lerp(Vector) (Variables|Default|GetStart%20Location) (Variables|Default|GetEnd%20Location) _value) false false))
    (:Finished
      (switch Utilities|FlowControl|Switch|SwitchonETimelineDirection _direction
        (:Forward
          (CallFunction|PlayRW))
        (:Backward
          (CallFunction|PlayFW))))))

(fn ConstructionScript)

(fn GetEndLocation
  (params (Direction :type Float%20%28double-precision%29))
  (return (+ (Variables|Default|GetStart%20Location) (* (* (Variables|Default|GetMovement%20Direction) Direction) (Variables|Default|GetMultiplier)))))